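; BP_GunBase is a gun base Blueprint that, in this graph, only shows the local player an on-screen ammo readout.
; Each Tick, on remote (non-authority) instances only, it checks that the owning pawn is controlled by the first local player controller.
; In deploying, idle, firing, reloading or holstering states, it prints the weapon name and clip count against a hardcoded capacity for one frame.
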(event `self.ReceiveTick`
  (params (DeltaSeconds :type "Float (single-precision)"))
  (`|ExecutionSequence`
    (:`then_0`
      (`/Engine/EditorBlueprintResources/ActorMacros.Switch Has Authority`
        (:`Remote`
          (bind _aspawn (cast `Pawn` (`self.GetOwner`)))
          (if (== (`Pawn.GetController` _aspawn) (`GameplayStatics.GetPlayerController` 0))
            (switch `EWeaponState` (`self.State`)
              (:`Deploying`
                _)
              (:`Idle`
                _)
              (:`Firing`
                _)
              (:`Reloading`
                _)
              (:`Holstering`
                _))
            (`KismetSystemLibrary.PrintText` (`|FormatText` "{Weapon} {Clip} / 30" (`self.Name`) (`self.Clip`)) true true (struct :`G` 0.66 :`B` 1.0 :`A` 1.0) DeltaSeconds)))))))

(fn `UserConstructionScript`)